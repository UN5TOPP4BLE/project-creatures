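; Boss-fight lever that the player pulls while overlapping its box, provided its LeverNumber is within one of the player's PhaseNumber.
; A pull tilts the lever by timeline and, for non-fence walls, sends particle actors flying to them.
; On first use it swaps Walls in and PreviousWalls out by visibility and height, then updates the phase.
; Gradual wall movement is disconnected, though LoadSwitched still applies Move offsets when restoring switched state.
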(event OnComponentBeginOverlap(BoxCollision)
  (params (OverlappedComponent :type Primitive%20Component%20Object%20Reference) (OtherActor :type Actor%20Object%20Reference) (OtherComp :type Primitive%20Component%20Object%20Reference) (OtherBodyIndex :type Integer) (bFromSweep :type Boolean) (SweepResult :type Hit%20Result%20Structure%20%28by%20ref%29))
  (bind _walls (Variables|Default|GetWalls))
  (bind _output (Utilities|Array|Get(acopy) _walls))
  (Utilities|Casting|CastToBP_ThirdPersonCharacter OtherActor)
  (if (not (Variables|Default|GetIsOverlapping?))
    (Variables|Default|SetIsOverlapping? true)
    ;[1 1 1] Add and remove text from screen
    (Development|PrintString "BEGIN")
    (Development|PrintString (Utilities|GetDisplayName OtherComp))
    (bind _returnvalue (UserInterface|CreateWidget "/Game/ui/WBP_Interact.WBP_Interact_C"))
    (Variables|/Game/ui/WBP_Interact.WBP_Interact_C|SetisGrey _returnvalue true)
    (bind _output_get (Variables|Default|SetWidget _returnvalue))
    (UserInterface|Viewport|AddtoViewport _output_get 0)
    (Utilities|FlowControl|Gate true) ; enters at Open
  ))

(event OnComponentEndOverlap(BoxCollision)
  (params (OverlappedComponent :type Primitive%20Component%20Object%20Reference) (OtherActor :type Actor%20Object%20Reference) (OtherComp :type Primitive%20Component%20Object%20Reference) (OtherBodyIndex :type Integer))
  (bind _walls (Variables|Default|GetWalls))
  (bind _output (Utilities|Array|Get(acopy) _walls))
  (Utilities|Casting|CastToBP_ThirdPersonCharacter OtherActor)
  (Variables|Default|SetIsOverlapping? false)
  ;[1 1 1] Add and remove text from screen
  (Development|PrintString "END")
  (Development|PrintString (Utilities|GetDisplayName OtherComp))
  (Widget|RemovefromParent (Variables|Default|GetWidget))
  (Utilities|FlowControl|Gate true) ; enters at Close
)

(event Custom|OneOfObjectsEndsMoving
  (bind _widget (Variables|Default|GetWidget))
  (if (not false)
    (Utilities|IsValid _widget
      (:Is%20Valid
        (Variables|/Game/ui/WBP_Interact.WBP_Interact_C|SetisGrey _widget false)))))

(event Custom|MoveParticleEmitter
  (params (PE :type Actor%20Object%20Reference) (TimelineTrack :type Float%20%28double-precision%29) (FinalLocation :type Vector) (StartLocation :type Vector))
  (Rendering|SetActorHiddenInGame PE false)
  (Transformation|SetActorLocation PE (Math|Vector|Lerp(Vector) StartLocation FinalLocation TimelineTrack) false false))

(event Custom|StartParticleEmitterTimeline
  (bind _particleemitters (Variables|Default|GetParticleEmitters))
  (bind _initialpositionparticleemitter (Variables|Default|GetInitialPositionParticleEmitter))
  (bind _alpha (Timeline|ParticleEmitterTimeline PlayFromStart)
    (:Update
      (for (_array_element _array_index) _particleemitters
        (CallFunction|MoveParticleEmitter _array_element _alpha (Transformation|GetActorLocation (Utilities|Array|Get(acopy) (Variables|Default|GetWalls) _array_index)) _initialpositionparticleemitter)))
    (:Finished
      (Rendering|SetActorHiddenInGame _particleemitters true)
      (for _array_element_2 _particleemitters
        (Transformation|SetActorLocation _array_element_2 _initialpositionparticleemitter false false)))))

(event EventBeginPlay
  (bind _returnvalue (Transformation|GetActorLocation))
  (Input|EnableInput (Game|GetPlayerController 0))
  (for _array_element (Variables|Default|GetWalls)
    (Utilities|Array|Add (Variables|Default|GetStartLocations) (Transformation|GetActorLocation _array_element))
    (bind _returnvalue_2 (Game|SpawnActorfromClass "/Game/Graphics/LeverParticles_BP.LeverParticles_BP_C" (Math|Conversions|ToTransform(Vector) _returnvalue) "Undefined" 0 0))
    (Rendering|SetActorHiddenInGame _returnvalue_2 true)
    (Utilities|Array|AppendArray (Variables|Default|GetParticleEmitters) (Utilities|Array|MakeArray _returnvalue_2))
    (Variables|Default|SetInitialPositionParticleEmitter _returnvalue)))

(event Input|ActionEvents|InputActionInteract
  (params (Key :type Key%20Structure :default "None"))
  (bind _widget (Variables|Default|GetWidget))
  (bind _walls (Variables|Default|GetWalls))
  (bind _output (Utilities|Array|Get(acopy) _walls))
  (:Pressed
    (if (not (Variables|Default|GetisMoving))
      (bind _asbp_third_person_character (Utilities|Casting|CastToBP_ThirdPersonCharacter (Game|GetPlayerCharacter 0)))
      (if (not (> (Math|Integer|Absolute(Integer) (- (Variables|Default|GetleverNumber) (Variables|/Game/ThirdPerson/Blueprints/BP_ThirdPersonCharacter.BP_ThirdPersonCharacter_C|GetphaseNumber _asbp_third_person_character))) 1))
        (Utilities|IsValid _widget
          (:Is%20Valid
            (Variables|/Game/ui/WBP_Interact.WBP_Interact_C|SetisGrey _widget true)
            (Utilities|FlowControl|Gate true
              (:Exit
                (Development|PrintString (Utilities|GetObjectName self))
                (for _array_element (Variables|Default|GetWalls)
                  _)
                (Variables|Default|SetSwitched (not (Variables|Default|GetSwitched)))
                (Variables|Default|SetisMoving true)
                ;[1 1 1] Check if walls are fences - if not then start particle emitter timeline
                (Utilities|Casting|CastToBP_FenceMoveable _output
                  (:then
                    _)
                  (:CastFailed
                    (Utilities|Casting|CastToBP_FenceMoveableWood _output
                      (:then
                        _)
                      (:CastFailed
                        (CallFunction|StartParticleEmitterTimeline)))))
                ;[1 1 1] Move lever
                (Audio|PlaySoundatLocation "/Game/Sounds/Footsteps/General/LeverPullSoundCue.LeverPullSoundCue" "0, 0, 0" "0, 0, 0" 1.0 1.0 0.0 0 0 0 0)
                (Components|Timeline|SetPlayRate (Variables|Default|GetTimelineLever) 1.0)
                (if (Variables|Default|GetSwitched)
                  (bind _lever (Timeline|TimelineLever PlayFromStart)
                    (:Update
                      (Transformation|SetRelativeRotation (Variables|Default|GetCenter) (Math|Rotator|MakeRotator (Math|Float|Lerp -3e+01 3e+01 _lever) 0.0 0.0) false false))
                    (:Finished
                      (Components|Timeline|SetPlayRate (Variables|Default|GetTimelineWalls) (/ 1.0 (Variables|Default|GetTime)))
                      (Audio|PlaySoundatLocation "/Game/Sounds/Footsteps/General/PlatformMoveSoundCue.PlatformMoveSoundCue" "0, 0, 0" "0, 0, 0" 1.0 1.0 0.0 0 0 0 0)
                      (if (Variables|Default|GetSwitched)
                        ;[1 1 1] Set start locations
                        (for (_array_element_2 _array_index) (Variables|Default|GetWalls)
                          (Utilities|Array|SetArrayElem (Variables|Default|GetStartLocations) _array_index (Transformation|GetActorLocation _array_element_2)))
                        (else
                          (for (_array_element_3 _array_index_2) (Variables|Default|GetWalls)
                            _)))
                      (Variables|Default|SetisMoving false)
                      (Variables|/Game/ui/WBP_Interact.WBP_Interact_C|SetisGrey (Variables|Default|GetWidget) false)
                      (if (not (> (Variables|Default|GetUsageNumber) 0))
                        (Variables|Default|SetUsageNumber 1)
                        (for _array_element_4 (Variables|Default|GetWalls)
                          (Rendering|SetActorHiddenInGame _array_element_4 false)
                          (Transformation|SetActorLocation _array_element_4 (Math|Vector|MakeVector (.x (Transformation|GetActorLocation _array_element_4)) (.y (Transformation|GetActorLocation _array_element_4)) (+ (.z (Transformation|GetActorLocation _array_element_4)) 1e+03)) false false))
                        (for _array_element_5 (Variables|Default|GetPreviousWalls)
                          (Rendering|SetActorHiddenInGame _array_element_5 true)
                          (Transformation|SetActorLocation _array_element_5 (Math|Vector|MakeVector (.x (Transformation|GetActorLocation _array_element_5)) (.y (Transformation|GetActorLocation _array_element_5)) (- (.z (Transformation|GetActorLocation _array_element_5)) 1e+03)) false false))
                        (bind _asbp_third_person_character_2 (Utilities|Casting|CastToBP_ThirdPersonCharacter (Game|GetPlayerCharacter 0)))
                        (bind _output_get (Variables|/Game/ThirdPerson/Blueprints/BP_ThirdPersonCharacter.BP_ThirdPersonCharacter_C|SetphaseNumber _asbp_third_person_character_2 (Variables|Default|GetleverNumber)))
                        (Development|PrintString (Utilities|String|ToString(Integer) _output_get)))))
                  (else
                    (Timeline|TimelineLever ReverseFromEnd)))))))))))

(fn ConstructionScript)

(fn MoveWall
  (params (Wall :type Actor%20Object%20Reference) (Vector :type Vector) (Move :type Vector) (StartLocation :type Vector))
  (bind (_x _y _z) (Math|Vector|BreakVector Move))
  (bind (_x_2 _y_2 _z_2) (Math|Vector|BreakVector Vector))
  (Transformation|SetActorLocation Wall (+ (Math|Vector|MakeVector (* _x_2 _x) (* _y_2 _y) (* _z_2 _z)) StartLocation) false false))

(fn CheckifObjectsAreMoving
  (return false))

(fn LoadSwitched
  (params (isSwitched :type Boolean))
  (Variables|Default|SetSwitched isSwitched)
  (if isSwitched
    (Transformation|SetRelativeRotation (Variables|Default|GetCenter) (Math|Rotator|MakeRotator 3e+01 0.0 0.0) false false)
    (for (_array_element _array_index) (Variables|Default|GetWalls)
      (Transformation|SetActorLocation _array_element (+ (Transformation|GetActorLocation _array_element) (Utilities|Array|Get(acopy) (Variables|Default|GetMove) _array_index)) false false)
      (Development|PrintString "MOVE")
      (Development|PrintString (Utilities|GetObjectName _array_element))
      (Development|PrintString (Utilities|String|ToString(Vector) (Utilities|Array|Get(acopy) (Variables|Default|GetMove) _array_index)))
      (Development|PrintString "--------------"))))