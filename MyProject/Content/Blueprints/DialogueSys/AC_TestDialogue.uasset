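; Test dialogue component that scripts a branching conversation with a Frog NPC by overriding the parent's Dialogue function.
; A switch on DialogueTreeIndex picks between first meeting, reminder and small-talk branches, each built from AddDialogue nodes that branch on the chosen option.
; Choices set the tree index before closing the conversation, and the introduction line is shared between branches.
; The small-talk branch randomizes its reply option and clears dialogue progress before closing.
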(event EventBeginPlay)

(event EventTick
  (params (DeltaSeconds :type Float%20%28single-precision%29)))

(fn Dialogue
  (|CallParentFunction)
  (switch int (Variables|Default|GetDialogueTreeIndex)
    (:0
      (bind (_state _optionindex) (CallFunction|AddDialogue "Frog" "Oh, hi there! Didn't seen you in a while." (Utilities|Array|MakeArray "Yeah, long time no see!" "Who are you again?")))
      (switch Utilities|FlowControl|Switch|SwitchonEnum_DialogueState _state
        (:NewEnumerator0
          (switch int _optionindex
            (:0
              (CallFunction|SetDialogueTreeIndex 2))
            (:1
              (bind _state_2 (CallFunction|AddDialogue "Frog" "I am your faithful friend - Frog! I will help you on your journey!" (Utilities|Array|MakeArray "Oh, thanks, Frog!") :!label _label))
              (switch Utilities|FlowControl|Switch|SwitchonEnum_DialogueState _state_2
                (:NewEnumerator0
                  (CallFunction|SetDialogueTreeIndex 1)))))
          (CallFunction|CloseConversation))))
    (:1
      (bind (_state_3 _optionindex_2) (CallFunction|AddDialogue "Frog" "Do you remember me now?" (Utilities|Array|MakeArray "Yeah, thanks for filling in!!" "Can you please repeat again?")))
      (switch Utilities|FlowControl|Switch|SwitchonEnum_DialogueState _state_3
        (:NewEnumerator0
          (switch int _optionindex_2
            (:0
              (CallFunction|SetDialogueTreeIndex 2)
              (CallFunction|CloseConversation))
            (:1
              (goto _label))))))
    (:2
      (bind _state_4 (CallFunction|AddDialogue "Frog" "So what are you on about?" (Utilities|Array|MakeArray (Utilities|Select :Index (Math|Random|RandomIntegerinRange 0 1) :Option%200 "Just checking!" :Option%201 "Nevermind!"))))
      (switch Utilities|FlowControl|Switch|SwitchonEnum_DialogueState _state_4
        (:NewEnumerator0
          (CallFunction|ClearDialogueProgress)
          (CallFunction|CloseConversation))))))