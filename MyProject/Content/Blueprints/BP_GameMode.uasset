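; Game mode that saves and restores progress through a single save slot.
; BeginPlay creates the save or, when its saved-location flag is set, restores player transform, wand possession (destroying world wands if held) and lever states.
; SaveGame records that state, pairing lever states to actors by sorted array index.
; LoadGame restarts the level, RestartLevel deletes the save first, and ChangeLevels clears the saved-location flag.
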(event Custom|Save%20Game
  (bind _leversswitched (Variables|Default|GetLeversSwitched))
  ;[1 1 1] Save game
  (bind _returnvalue (SaveGame|LoadGamefromSlot "save1"))
  (bind _asbp_save_game (Utilities|Casting|CastToBP_SaveGame _returnvalue))
  (bind _asbp_third_person_character (Utilities|Casting|CastToBP_ThirdPersonCharacter (Game|GetPlayerCharacter 0)))
  (Variables|/Game/Blueprints/BP_SaveGame.BP_SaveGame_C|SetCharTransform _asbp_save_game (Transformation|GetActorTransform _asbp_third_person_character))
  (Variables|/Game/Blueprints/BP_SaveGame.BP_SaveGame_C|SetUseSavedLocation _asbp_save_game true)
  (Variables|/Game/Blueprints/BP_SaveGame.BP_SaveGame_C|SethasWand _asbp_save_game (Variables|/Game/ThirdPerson/Blueprints/BP_ThirdPersonCharacter.BP_ThirdPersonCharacter_C|GethasWand _asbp_third_person_character))
  (bind _outactors (Actor|GetAllActorsOfClass "/Game/Blueprints/BP_Lever.BP_Lever_C"))
  (bind _output_get (Variables|Default|SetLevers _outactors))
  (bind _returnvalue_2 (Class|MyBlueprintFunctionLibrary|Sort _output_get))
  (for _array_element _returnvalue_2
    (bind _asbp_lever (Utilities|Casting|CastToBP_Lever _array_element))
    (Utilities|Array|Add _leversswitched (Variables|/Game/Blueprints/BP_Lever.BP_Lever_C|GetSwitched _asbp_lever))
    (Development|PrintString (Utilities|GetObjectName _asbp_lever)))
  (Variables|/Game/Blueprints/BP_SaveGame.BP_SaveGame_C|SetLevers _asbp_save_game _leversswitched)
  (SaveGame|SaveGametoSlot _asbp_save_game "save1"))

(event Custom|Load%20Game
  ;[1 1 1] Load Game
  (Development|ExecuteConsoleCommand "RestartLevel" 0))

(event Custom|RestartLevel
  ;[1 1 1] Delete save + Restart
  (SaveGame|DeleteGameinSlot "save1")
  (Development|ExecuteConsoleCommand "RestartLevel" 0))

(event Custom|ChangeLevels
  ;[1 1 1] Change Levels
  (bind _returnvalue (SaveGame|LoadGamefromSlot "save1"))
  (bind _asbp_save_game (Utilities|Casting|CastToBP_SaveGame _returnvalue))
  (Variables|/Game/Blueprints/BP_SaveGame.BP_SaveGame_C|SetUseSavedLocation _asbp_save_game false)
  (SaveGame|SaveGametoSlot _asbp_save_game "save1"))

(event EventBeginPlay
  (bind _returnvalue (SaveGame|DoesSaveGameExist "save1"))
  (if _returnvalue
    (bind _returnvalue_2 (SaveGame|LoadGamefromSlot "save1"))
    (bind _asbp_save_game (Utilities|Casting|CastToBP_SaveGame _returnvalue_2))
    (if (Variables|/Game/Blueprints/BP_SaveGame.BP_SaveGame_C|GetUseSavedLocation _asbp_save_game)
      ;[1 1 1] Load Game
      (bind _asbp_third_person_character (Utilities|Casting|CastToBP_ThirdPersonCharacter (Game|GetPlayerCharacter 0)))
      (Transformation|SetWorldTransform (Variables|/Script/Engine.Actor|GetRootComponent _asbp_third_person_character) (Variables|/Game/Blueprints/BP_SaveGame.BP_SaveGame_C|GetCharTransform _asbp_save_game) false false)
      (bind _output_get (Variables|/Game/ThirdPerson/Blueprints/BP_ThirdPersonCharacter.BP_ThirdPersonCharacter_C|SethasWand _asbp_third_person_character (Variables|/Game/Blueprints/BP_SaveGame.BP_SaveGame_C|GethasWand _asbp_save_game)))
      (if _output_get
        (bind _outactors (Actor|GetAllActorsOfClass "/Game/Blueprints/BP_Wand.BP_Wand_C"))
        (for _array_element _outactors
          (Actor|DestroyActor _array_element)))
      (bind _outactors_2 (Actor|GetAllActorsOfClass "/Game/Blueprints/BP_Lever.BP_Lever_C"))
      (bind _output_get_2 (Variables|Default|SetLevers _outactors_2))
      (bind _returnvalue_3 (Class|MyBlueprintFunctionLibrary|Sort _output_get_2))
      (for (_array_element_2 _array_index) _returnvalue_3
        (bind _asbp_lever (Utilities|Casting|CastToBP_Lever _array_element_2))
        (Development|PrintString (Utilities|GetObjectName _asbp_lever))
        (Default|LoadSwitched _asbp_lever (Utilities|Array|Get(acopy) (Variables|/Game/Blueprints/BP_SaveGame.BP_SaveGame_C|GetLevers _asbp_save_game) _array_index))
        (Utilities|Array|AddUnique (Variables|Default|GetWalls) 0)))
    (else
      ;[1 1 1] Create Save File
      (bind _returnvalue_4 (SaveGame|CreateSaveGameObject "/Game/Blueprints/BP_SaveGame.BP_SaveGame_C"))
      (SaveGame|SaveGametoSlot _returnvalue_4 "save1"))))

(event EventTick
  (params (DeltaSeconds :type Float%20%28single-precision%29)))

(fn ConstructionScript)