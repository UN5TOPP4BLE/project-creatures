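; BP_Checkpoint is a single-use checkpoint that saves the game when anything overlaps its Box.
; On overlap it adds itself to CheckpointUsed in the "save1" BP_SaveGame, writes the slot, calls SaveGame on BP_GameMode, then destroys itself.
; On BeginPlay it reloads that slot and destroys itself if already listed, so used checkpoints stay gone.
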(event OnComponentBeginOverlap(Box)
  (params (OverlappedComponent :type Primitive%20Component%20Object%20Reference) (OtherActor :type Actor%20Object%20Reference) (OtherComp :type Primitive%20Component%20Object%20Reference) (OtherBodyIndex :type Integer) (bFromSweep :type Boolean) (SweepResult :type Hit%20Result%20Structure%20%28by%20ref%29))
  (bind _returnvalue (SaveGame|LoadGamefromSlot "save1"))
  (bind _asbp_save_game (Utilities|Casting|CastToBP_SaveGame _returnvalue))
  (if (not (Utilities|Array|ContainsItem (Variables|/Game/Blueprints/BP_SaveGame.BP_SaveGame_C|GetCheckpointUsed _asbp_save_game) self))
    (Utilities|Array|Add (Variables|/Game/Blueprints/BP_SaveGame.BP_SaveGame_C|GetCheckpointUsed _asbp_save_game) self)
    (SaveGame|SaveGametoSlot _asbp_save_game "save1")
    (bind _asbp_game_mode (Utilities|Casting|CastToBP_GameMode (Game|GetGameMode)))
    (Default|SaveGame _asbp_game_mode)
    (Actor|DestroyActor)))

(event EventBeginPlay
  (bind _returnvalue (SaveGame|LoadGamefromSlot "save1"))
  (bind _asbp_save_game (Utilities|Casting|CastToBP_SaveGame _returnvalue))
  (if (Utilities|Array|ContainsItem (Variables|/Game/Blueprints/BP_SaveGame.BP_SaveGame_C|GetCheckpointUsed _asbp_save_game) self)
    (Actor|DestroyActor)))

(event Collision|EventActorBeginOverlap
  (params (OtherActor :type Actor%20Object%20Reference)))

(event EventTick
  (params (DeltaSeconds :type Float%20%28single-precision%29)))

(fn ConstructionScript)