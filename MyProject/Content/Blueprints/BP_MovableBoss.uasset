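; BP_MovableBoss moves its owning actor back and forth between a start and an end position, starting from the start position on BeginPlay.
; Tick accumulates elapsed time and calls Move, which sets the location by interpolating between both points with a float curve sampled at elapsed over total time.
; When the actor comes within a small distance of its target, Move flips the direction and resets the timer.
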(event EventBeginPlay
  (Transformation|SetActorLocation (Components|GetOwner) (Variables|Default|GetStartPosition) false false))

(event EventTick
  (params (DeltaSeconds :type Float%20%28single-precision%29))
  (bind _returnvalue (Components|GetOwner))
  (bind _startposition (Variables|Default|GetStartPosition))
  (bind _endposition (Variables|Default|GetEndPosition))
  (Variables|Default|SetcurrentTime (+ DeltaSeconds (Variables|Default|GetcurrentTime)))
  (if (Variables|Default|GetGoingForward)
    (CallFunction|Move _returnvalue _startposition _endposition)
    (else
      (CallFunction|Move _returnvalue _endposition _startposition))))

(fn Move
  (params (movedActor :type Actor%20Object%20Reference) (beginningLocation :type Vector) (targetLocation :type Vector))
  (if (<= (Math|Vector|VectorLength (- targetLocation (Transformation|GetActorLocation movedActor))) 5.0)
    (Variables|Default|SetGoingForward (not (Variables|Default|GetGoingForward)))
    (Variables|Default|SetcurrentTime 0.0)
    (else
      (Transformation|SetActorLocation movedActor (+ beginningLocation (* (- targetLocation beginningLocation) (Math|Curves|GetFloatValue (Variables|Default|GetCurve) (/ (Variables|Default|GetcurrentTime) (Variables|Default|GetTime))))) false false))))