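; Pressure plate that moves the Cube of a linked ScianaP wall while something stands on it.
; Box overlaps not tagged NieKlikam are counted, so the button sinks on the first arrival and rises on the last exit.
; A timeline, rate-scaled by CzasTrwania, drives the wall's relative offset by per-axis Move values without sweep.
; On release it reverses, or stops if the Ruch motion flag is still set.
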(event OnComponentBeginOverlap(Box)
  (params (OverlappedComponent :type Primitive%20Component%20Object%20Reference) (OtherActor :type Actor%20Object%20Reference) (OtherComp :type Primitive%20Component%20Object%20Reference) (OtherBodyIndex :type Integer) (bFromSweep :type Boolean) (SweepResult :type Hit%20Result%20Structure%20%28by%20ref%29))
  (bind _przycisk (Variables|Default|GetPrzycisk))
  (bind _returnvalue (Transformation|GetWorldLocation _przycisk))
  (if (not (Components|ComponentHasTag OtherComp "NieKlikam"))
    (bind _result (Math|Integer|IncrementInt (Variables|Default|Getusers_count))
      (:%20%20
        (Development|PrintString (Utilities|String|ToString(Integer) _result))
        (if (== (Variables|Default|Getusers_count) 1)
          (Transformation|SetWorldLocation (Variables|Default|GetPrzycisk) (Math|Vector|MakeVector (.x _returnvalue) (.y _returnvalue) (- (.z _returnvalue) 4.0)) false false)
          (Variables|Default|SetRuch true)
          (Components|Timeline|SetPlayRate (Variables|Default|GetTimeline_1) (/ 1.0 (Variables|Default|GetCzas%20trwania)))
          (bind _newtrack_1 (Timeline|Timeline_1 Play)
            (:Update
              (Transformation|SetRelativeLocation (Variables|/Game/Blueprints/ScianaPrzenikalna.ScianaPrzenikalna_C|GetCube (Variables|Default|GetScianaP)) (Math|Vector|MakeVector (* (.X (Math|Vector|BreakVector _newtrack_1)) (Variables|Default|GetmoveX)) (* (.Y (Math|Vector|BreakVector _newtrack_1)) (Variables|Default|GetmoveY)) (* (.Z (Math|Vector|BreakVector _newtrack_1)) (Variables|Default|GetmoveZ))) false false)
              (Variables|Default|SetRuch false))))))))

(event OnComponentEndOverlap(Box)
  (params (OverlappedComponent :type Primitive%20Component%20Object%20Reference) (OtherActor :type Actor%20Object%20Reference) (OtherComp :type Primitive%20Component%20Object%20Reference) (OtherBodyIndex :type Integer))
  (bind _przycisk (Variables|Default|GetPrzycisk))
  (bind _users_count (Variables|Default|Getusers_count))
  (bind _returnvalue (Transformation|GetWorldLocation _przycisk))
  (if (not (Components|ComponentHasTag OtherComp "NieKlikam"))
    (bind _result (Math|Integer|DecrementInt _users_count)
      (:%20%20
        (Development|PrintString (Utilities|String|ToString(Integer) _result))
        (if (== _users_count 0)
          (Transformation|SetWorldLocation (Variables|Default|GetPrzycisk) (Math|Vector|MakeVector (.x _returnvalue) (.y _returnvalue) (+ (.z _returnvalue) 4.0)) false false)
          (if (Variables|Default|GetRuch)
            (bind _newtrack_1 (Timeline|Timeline_1 Stop)
              (:Update
                (Transformation|SetRelativeLocation (Variables|/Game/Blueprints/ScianaPrzenikalna.ScianaPrzenikalna_C|GetCube (Variables|Default|GetScianaP)) (Math|Vector|MakeVector (* (.X (Math|Vector|BreakVector _newtrack_1)) (Variables|Default|GetmoveX)) (* (.Y (Math|Vector|BreakVector _newtrack_1)) (Variables|Default|GetmoveY)) (* (.Z (Math|Vector|BreakVector _newtrack_1)) (Variables|Default|GetmoveZ))) false false)
                (Variables|Default|SetRuch false)))
            (else
              (Variables|Default|SetRuch true)
              (Timeline|Timeline_1 Reverse))))))))

(fn ConstructionScript)