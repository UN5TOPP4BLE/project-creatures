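; Pressure plate that moves an array of wall actors when stepped on.
; Box overlaps keep a count of components lacking the "NieKlikam" tag; the first lowers the button and plays a timeline, with play rate set from CzasTrwania.
; The timeline's vector track scales per-wall offsets added to locations cached at BeginPlay.
; Unless IsOneTime, the last exit raises the button and reverses the timeline, or stops it if Ruch is set.
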(event OnComponentBeginOverlap(Box)
  (params (OverlappedComponent :type Primitive%20Component%20Object%20Reference) (OtherActor :type Actor%20Object%20Reference) (OtherComp :type Primitive%20Component%20Object%20Reference) (OtherBodyIndex :type Integer) (bFromSweep :type Boolean) (SweepResult :type Hit%20Result%20Structure%20%28by%20ref%29))
  (bind _przycisk (Variables|Default|GetPrzycisk))
  (bind _returnvalue (Transformation|GetWorldLocation _przycisk))
  (if (not (Components|ComponentHasTag OtherComp "NieKlikam"))
    (bind _result (Math|Integer|IncrementInt (Variables|Default|Getusers_count))
      (:%20%20
        (Development|PrintString (Utilities|String|ToString(Integer) _result))
        (if (== (Variables|Default|Getusers_count) 1)
          (Transformation|SetWorldLocation (Variables|Default|GetPrzycisk) (Math|Vector|MakeVector (.x _returnvalue) (.y _returnvalue) (- (.z _returnvalue) 4.0)) false false)
          (Variables|Default|SetRuch true)
          (Components|Timeline|SetPlayRate (Variables|Default|GetTimeline_1) (/ 1.0 (Variables|Default|GetCzas%20trwania)))
          (bind _newtrack_1 (Timeline|Timeline_1 Play)
            (:Update
              (for (_array_element _array_index) (Variables|Default|GetWalls)
                (CallFunction|MoveWall _array_element _newtrack_1 (Utilities|Array|Get(acopy) (Variables|Default|GetMove) _array_index) (Utilities|Array|Get(acopy) (Variables|Default|GetStartLocations) _array_index)))
              (Variables|Default|SetRuch false))))))))

(event OnComponentEndOverlap(Box)
  (params (OverlappedComponent :type Primitive%20Component%20Object%20Reference) (OtherActor :type Actor%20Object%20Reference) (OtherComp :type Primitive%20Component%20Object%20Reference) (OtherBodyIndex :type Integer))
  (bind _przycisk (Variables|Default|GetPrzycisk))
  (bind _users_count (Variables|Default|Getusers_count))
  (bind _returnvalue (Transformation|GetWorldLocation _przycisk))
  (if (not (Variables|Default|GetisOneTime))
    (if (not (Components|ComponentHasTag OtherComp "NieKlikam"))
      (Math|Integer|DecrementInt _users_count
        (:%20%20
          (if (== _users_count 0)
            (Transformation|SetWorldLocation (Variables|Default|GetPrzycisk) (Math|Vector|MakeVector (.x _returnvalue) (.y _returnvalue) (+ (.z _returnvalue) 4.0)) false false)
            (if (Variables|Default|GetRuch)
              (bind _newtrack_1 (Timeline|Timeline_1 Stop)
                (:Update
                  (for (_array_element _array_index) (Variables|Default|GetWalls)
                    (CallFunction|MoveWall _array_element _newtrack_1 (Utilities|Array|Get(acopy) (Variables|Default|GetMove) _array_index) (Utilities|Array|Get(acopy) (Variables|Default|GetStartLocations) _array_index)))
                  (Variables|Default|SetRuch false)))
              (else
                (Variables|Default|SetRuch true)
                (Timeline|Timeline_1 Reverse)))))))))

(event EventBeginPlay
  (for _array_element (Variables|Default|GetWalls)
    (Utilities|Array|Add (Variables|Default|GetStartLocations) (Transformation|GetActorLocation _array_element))))

(fn ConstructionScript)

(fn MoveWall
  (params (Wall :type Actor%20Object%20Reference) (Vector :type Vector) (Move :type Vector) (StartLocation :type Vector))
  (bind (_x _y _z) (Math|Vector|BreakVector Move))
  (bind (_x_2 _y_2 _z_2) (Math|Vector|BreakVector Vector))
  (Transformation|SetActorLocation Wall (+ (Math|Vector|MakeVector (* _x_2 _x) (* _y_2 _y) (* _z_2 _z)) StartLocation) false false))