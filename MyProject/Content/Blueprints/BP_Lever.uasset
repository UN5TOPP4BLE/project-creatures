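; Interactable lever that toggles a set of walls between two positions.
; Overlapping its box as the third-person character shows an interact widget and opens a Gate for the Interact input.
; Each press flips Switched, playing or reversing a timeline that rotates the lever.
; When that finishes, a second timeline, rate-scaled by Time, moves each wall's cube along its own Move vector, forward or back.
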(event OnComponentBeginOverlap(BoxCollision)
  (params (OverlappedComponent :type Primitive%20Component%20Object%20Reference) (OtherActor :type Actor%20Object%20Reference) (OtherComp :type Primitive%20Component%20Object%20Reference) (OtherBodyIndex :type Integer) (bFromSweep :type Boolean) (SweepResult :type Hit%20Result%20Structure%20%28by%20ref%29))
  (Utilities|Casting|CastToBP_ThirdPersonCharacter OtherActor)
  ;[1 1 1] Add and remove text from screen
  (bind _returnvalue (UserInterface|CreateWidget "/Game/ui/WBP_Interact.WBP_Interact_C"))
  (UserInterface|Viewport|AddtoViewport _returnvalue 0)
  (Utilities|FlowControl|Gate true) ; enters at Open
)

(event OnComponentEndOverlap(BoxCollision)
  (params (OverlappedComponent :type Primitive%20Component%20Object%20Reference) (OtherActor :type Actor%20Object%20Reference) (OtherComp :type Primitive%20Component%20Object%20Reference) (OtherBodyIndex :type Integer))
  (Utilities|Casting|CastToBP_ThirdPersonCharacter OtherActor)
  ;[1 1 1] Add and remove text from screen
  (Widget|RemovefromParent (stale OnComponentBeginOverlap(BoxCollision) _returnvalue))
  (Utilities|FlowControl|Gate true) ; enters at Close
)

(event EventBeginPlay
  (Input|EnableInput (Game|GetPlayerController 0)))

(event Collision|EventActorBeginOverlap
  (params (OtherActor :type Actor%20Object%20Reference)))

(event EventTick
  (params (DeltaSeconds :type Float%20%28single-precision%29)))

(event Input|ActionEvents|InputActionInteract
  (params (Key :type Key%20Structure :default "None"))
  (:Pressed
    (Development|PrintString "Hello")
    (Variables|/Game/ui/WBP_Interact.WBP_Interact_C|SetisPressed (stale OnComponentBeginOverlap(BoxCollision) _returnvalue) true)
    (Utilities|FlowControl|Delay 0.3)
    (Variables|/Game/ui/WBP_Interact.WBP_Interact_C|SetisPressed (stale OnComponentBeginOverlap(BoxCollision) _returnvalue) false)
    (Utilities|FlowControl|Gate true
      (:Exit
        (Variables|Default|SetSwitched (not (Variables|Default|GetSwitched)))
        (Variables|Default|SetisMoving true)
        (Components|Timeline|SetPlayRate (Variables|Default|GetTimelineLever) 1.0)
        (if (Variables|Default|GetSwitched)
          (bind _lever (Timeline|TimelineLever Play)
            (:Update
              (Transformation|SetRelativeRotation (Variables|Default|GetCenter) (Math|Rotator|MakeRotator (Math|Float|Lerp -3e+01 3e+01 _lever) 0.0 0.0) false false))
            (:Finished
              (Components|Timeline|SetPlayRate (Variables|Default|GetTimelineWalls) (/ 1.0 (Variables|Default|GetTime)))
              (if (Variables|Default|GetSwitched)
                (bind _newtrack_0 (Timeline|TimelineWalls Play)
                  (:Update
                    (for (_array_element _array_index) (Variables|Default|GetWalls)
                      (CallFunction|MoveWall _array_element _newtrack_0 (Utilities|Array|Get(acopy) (Variables|Default|GetMove) _array_index)))
                    (Variables|Default|SetisMoving false)))
                (else
                  (Timeline|TimelineWalls Reverse)))))
          (else
            (Timeline|TimelineLever Reverse)))))))

(fn ConstructionScript)

(fn MoveWall
  (params (Wall :type Sciana%20Object%20Reference) (Vector :type Vector) (Move :type Vector))
  (bind (_x _y _z) (Math|Vector|BreakVector Move))
  (bind (_x_2 _y_2 _z_2) (Math|Vector|BreakVector Vector))
  (Transformation|SetRelativeLocation (Variables|/Game/Blueprints/Sciana.Sciana_C|GetCube Wall) (Math|Vector|MakeVector (* _x_2 _x) (* _y_2 _y) (* _z_2 _z)) false false))