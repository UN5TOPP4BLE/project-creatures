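; Creature manager component that tracks the player's creatures and switches which one is active with the 1 and 2 keys.
; Parallel arrays indexed by the active slot hold each creature's entry, created flag and spawned reference, with getters and setters for the current one.
; Switching stops every valid creature through its NPCController, then starts the selected one and notifies the owning BP_ThirdPersonCharacter if that reference is valid.
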(event Input|KeyboardEvents|1
  (params (Key :type Key%20Structure))
  (:Pressed
    (CallFunction|ChangeActiveCreature)))

(event Input|KeyboardEvents|2
  (params (Key :type Key%20Structure))
  (:Pressed
    (CallFunction|ChangeActiveCreature 1)))

(fn GetActiveCreature
  (return (Utilities|Array|Get(acopy) (Variables|Default|GetCreatures) (Variables|Default|GetActiveCreature))))

(fn CheckActiveCreatureCreated
  (return (Utilities|Array|Get(acopy) (Variables|Default|GetIsCreaturesCreated) (Variables|Default|GetActiveCreature))))

(fn SetActiveCreated
  (params (isCreated :type Boolean))
  (Utilities|Array|SetArrayElem (Variables|Default|GetIsCreaturesCreated) (Variables|Default|GetActiveCreature) isCreated))

(fn GetActiveCreatureReference
  (return (Utilities|Array|Get(acopy) (Variables|Default|GetCreaturesObjectReference) (Variables|Default|GetActiveCreature))))

(fn SetActiveCreatureReference
  (params (NewCharacter :type Character%20Object%20Reference))
  (Utilities|Array|SetArrayElem (Variables|Default|GetCreaturesObjectReference) (Variables|Default|GetActiveCreature) NewCharacter))

(fn ChangeActiveCreature
  (params (NewActiveCreatureNumber :type Integer))
  (Variables|Default|SetActiveCreature NewActiveCreatureNumber)
  (for _array_element (Variables|Default|GetCreaturesObjectReference)
    (if (Utilities|IsValid _array_element)
      (bind _asnpccontroller (Utilities|Casting|CastToNPCController (Pawn|GetController _array_element)))
      (Default|StopMoving _asnpccontroller)))
  (bind _activecreaturereference (CallFunction|GetActiveCreatureReference))
  (if (Utilities|IsValid _activecreaturereference)
    (bind _asnpccontroller_2 (Utilities|Casting|CastToNPCController (Pawn|GetController _activecreaturereference)))
    (Default|StartMoving _asnpccontroller_2)
    (bind _asbp_third_person_character (Utilities|Casting|CastToBP_ThirdPersonCharacter (Components|GetOwner)))
    (Default|CreatureChange _asbp_third_person_character)))