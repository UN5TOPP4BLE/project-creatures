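; BP_Puddle is a water area that tells the player character whether its lake destination or the frog NPC is on water.
; Tick polls NiebieskiBox and sets IsLakeOnWater for DestinationLake or TargetPoint, checking for an overlapping NPC only when neither is inside.
; End overlap clears the matching flag, treating the first NPC in the level as the frog.
; Begin-overlap events are empty, and older counting and debug logic is left disconnected.
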(event OnComponentBeginOverlap(NiebieskiBox)
  (params (OverlappedComponent :type Primitive%20Component%20Object%20Reference) (OtherActor :type Actor%20Object%20Reference) (OtherComp :type Primitive%20Component%20Object%20Reference) (OtherBodyIndex :type Integer) (bFromSweep :type Boolean) (SweepResult :type Hit%20Result%20Structure%20%28by%20ref%29)))

(event OnComponentEndOverlap(NiebieskiBox)
  (params (OverlappedComponent :type Primitive%20Component%20Object%20Reference) (OtherActor :type Actor%20Object%20Reference) (OtherComp :type Primitive%20Component%20Object%20Reference) (OtherBodyIndex :type Integer))
  (bind _asbp_third_person_character (Utilities|Casting|CastToBP_ThirdPersonCharacter (Game|GetPlayerCharacter 0)))
  (if (== (Variables|/Game/ThirdPerson/Blueprints/BP_ThirdPersonCharacter.BP_ThirdPersonCharacter_C|GetDestinationLake _asbp_third_person_character) OtherActor)
    (Variables|/Game/ThirdPerson/Blueprints/BP_ThirdPersonCharacter.BP_ThirdPersonCharacter_C|SetIsLakeOnWater? _asbp_third_person_character false :!label _label)
    (elif (== OtherActor (Variables|/Game/ThirdPerson/Blueprints/BP_ThirdPersonCharacter.BP_ThirdPersonCharacter_C|GetTargetPoint _asbp_third_person_character))
      (goto _label)
      (else
        (bind _outactors (Actor|GetAllActorsOfClass "/Game/NPC/NPC.NPC_C"))
        (if (== (Utilities|Array|Get(acopy) _outactors) OtherActor)
          (Development|PrintString "FROG NOT ON WATER")
          (Variables|/Game/ThirdPerson/Blueprints/BP_ThirdPersonCharacter.BP_ThirdPersonCharacter_C|SetIsFrogOnWater? _asbp_third_person_character false))))))

(event EventBeginPlay
  (bind _asbp_third_person_character (Utilities|Casting|CastToBP_ThirdPersonCharacter (Game|GetPlayerCharacter 0)))
  (Variables|Default|SetAs%20BP%20Third%20Person%20Character _asbp_third_person_character))

(event Collision|EventActorBeginOverlap
  (params (OtherActor :type Actor%20Object%20Reference)))

(event EventTick
  (params (DeltaSeconds :type Float%20%28single-precision%29))
  (bind _niebieskibox (Variables|Default|GetNiebieskiBox))
  (bind _as_bp_third_person_character (Variables|Default|GetAs%20BP%20Third%20Person%20Character))
  (bind _niebieskibox_2 (Variables|Default|GetNiebieskiBox))
  (bind _overlappingactors (Collision|GetOverlappingActors _niebieskibox_2 "/Game/NPC/NPC.NPC_C" :!class /Script/Engine.PrimitiveComponent))
  (if (Collision|IsOverlappingActor _niebieskibox (Variables|/Game/ThirdPerson/Blueprints/BP_ThirdPersonCharacter.BP_ThirdPersonCharacter_C|GetDestinationLake _as_bp_third_person_character) :!class /Script/Engine.PrimitiveComponent)
    (Variables|/Game/ThirdPerson/Blueprints/BP_ThirdPersonCharacter.BP_ThirdPersonCharacter_C|SetIsLakeOnWater? _as_bp_third_person_character true)
    (elif (Collision|IsOverlappingActor _niebieskibox (Variables|/Game/ThirdPerson/Blueprints/BP_ThirdPersonCharacter.BP_ThirdPersonCharacter_C|GetTargetPoint _as_bp_third_person_character) :!class /Script/Engine.PrimitiveComponent)
      (Variables|/Game/ThirdPerson/Blueprints/BP_ThirdPersonCharacter.BP_ThirdPersonCharacter_C|SetIsLakeOnWater? _as_bp_third_person_character true)
      (elif (>= (Utilities|Array|Length _overlappingactors) 1)
        (bind _asnpc (Utilities|Casting|CastToNPC (Utilities|Array|Get(acopy) _overlappingactors))
          (:then
            (if (Class|PrimitiveComponent|IsOverlappingComponent (Variables|/Script/Engine.Character|GetMesh _asnpc) (Variables|Default|GetNiebieskiBox))
              (Variables|/Game/ThirdPerson/Blueprints/BP_ThirdPersonCharacter.BP_ThirdPersonCharacter_C|SetIsFrogOnWater? _as_bp_third_person_character true :!label _label)))
          (:CastFailed
            (goto _label)))))))

(fn ConstructionScript)