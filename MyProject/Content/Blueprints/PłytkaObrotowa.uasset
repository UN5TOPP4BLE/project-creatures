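; Pressure plate (PłytkaObrotowa) that turns a linked Obracacz tile when something steps on it.
; Box overlaps count occupants, skipping components tagged NieKlikam and printing the count for debug.
; The first occupant lowers the Przycisk button and instantly yaws the Pole of the Obracacz at index NrPola in GetAllActorsOfClass by a quarter turn.
; The last one leaving raises the button without reversing the rotation.
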(event OnComponentBeginOverlap(Box)
  (params (OverlappedComponent :type Primitive%20Component%20Object%20Reference) (OtherActor :type Actor%20Object%20Reference) (OtherComp :type Primitive%20Component%20Object%20Reference) (OtherBodyIndex :type Integer) (bFromSweep :type Boolean) (SweepResult :type Hit%20Result%20Structure%20%28by%20ref%29))
  (bind _przycisk (Variables|Default|GetPrzycisk))
  (bind _returnvalue (Transformation|GetWorldLocation _przycisk))
  (if (not (Components|ComponentHasTag OtherComp "NieKlikam"))
    (bind _result (Math|Integer|IncrementInt (Variables|Default|Getusers_count))
      (:%20%20
        (Development|PrintString (Utilities|String|ToString(Integer) _result))
        (if (== (Variables|Default|Getusers_count) 1)
          (Transformation|SetWorldLocation (Variables|Default|GetPrzycisk) (Math|Vector|MakeVector (.x _returnvalue) (.y _returnvalue) (- (.z _returnvalue) 4.0)) false false)
          (Variables|Default|SetRuch true)
          (bind _outactors (Actor|GetAllActorsOfClass "/Game/Blueprints/Obracacz.Obracacz_C"))
          (Transformation|SetWorldRotation (Variables|/Game/Blueprints/Obracacz.Obracacz_C|GetPole (Utilities|Array|Get(acopy) _outactors (Variables|Default|GetNrPola))) (Math|Rotator|MakeRotator (.roll (Transformation|GetWorldRotation (Variables|/Game/Blueprints/Obracacz.Obracacz_C|GetPole (Utilities|Array|Get(acopy) _outactors (Variables|Default|GetNrPola))))) (.pitch (Transformation|GetWorldRotation (Variables|/Game/Blueprints/Obracacz.Obracacz_C|GetPole (Utilities|Array|Get(acopy) _outactors (Variables|Default|GetNrPola))))) (+ (.yaw (Transformation|GetWorldRotation (Variables|/Game/Blueprints/Obracacz.Obracacz_C|GetPole (Utilities|Array|Get(acopy) _outactors (Variables|Default|GetNrPola))))) 9e+01)) false false))))))

(event OnComponentEndOverlap(Box)
  (params (OverlappedComponent :type Primitive%20Component%20Object%20Reference) (OtherActor :type Actor%20Object%20Reference) (OtherComp :type Primitive%20Component%20Object%20Reference) (OtherBodyIndex :type Integer))
  (bind _przycisk (Variables|Default|GetPrzycisk))
  (bind _users_count (Variables|Default|Getusers_count))
  (bind _returnvalue (Transformation|GetWorldLocation _przycisk))
  (if (not (Components|ComponentHasTag OtherComp "NieKlikam"))
    (bind _result (Math|Integer|DecrementInt _users_count)
      (:%20%20
        (Development|PrintString (Utilities|String|ToString(Integer) _result))
        (if (== _users_count 0)
          (Transformation|SetWorldLocation (Variables|Default|GetPrzycisk) (Math|Vector|MakeVector (.x _returnvalue) (.y _returnvalue) (+ (.z _returnvalue) 4.0)) false false)
          (if (not (Variables|Default|GetRuch))
            (Variables|Default|SetRuch true)))))))

(fn ConstructionScript)