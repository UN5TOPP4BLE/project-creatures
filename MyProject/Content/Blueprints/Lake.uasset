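; Lake actor meant to chain numbered lakes, teleporting a stationary Frog NPC to the lake with the next ID.
; BeginPlay counts lakes; Tick moves the stopped, overlapping NPC to NextLakeLocation while LakeTeleporting is set, except on the last lake.
; Logic matching the player's TPTarget and setting NPC, flag and destination is disconnected, leaving both overlap events empty.
; TeleportAfterOverlap and other unwired fragments are leftover attempts and debug prints.
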(event OnComponentEndOverlap(Box)
  (params (OverlappedComponent :type Primitive%20Component%20Object%20Reference) (OtherActor :type Actor%20Object%20Reference) (OtherComp :type Primitive%20Component%20Object%20Reference) (OtherBodyIndex :type Integer)))

(event OnComponentBeginOverlap(Box)
  (params (OverlappedComponent :type Primitive%20Component%20Object%20Reference) (OtherActor :type Actor%20Object%20Reference) (OtherComp :type Primitive%20Component%20Object%20Reference) (OtherBodyIndex :type Integer) (bFromSweep :type Boolean) (SweepResult :type Hit%20Result%20Structure%20%28by%20ref%29)))

(event Custom|TeleportAfterOverlap
  ;[1 1 1] Previous Try At ComponentBeginOverlap - will delete later
  (bind _asbp_third_person_character (Utilities|Casting|CastToBP_ThirdPersonCharacter (Game|GetPlayerCharacter 0)))
  (Development|PrintString (Utilities|String|ToString(Vector) (Transformation|GetWorldLocation (Variables|Transformation|GetRootComponent))) true true "(R=1.000000,G=0.000000,B=0.024272,A=1.000000)" 5.0)
  (Development|PrintString (Utilities|String|ToString(Vector) (Variables|/Game/ThirdPerson/Blueprints/BP_ThirdPersonCharacter.BP_ThirdPersonCharacter_C|GetTPTarget _asbp_third_person_character)) true true "(R=0.000000,G=0.660000,B=1.000000,A=1.000000)" 5.0)
  (if true
    (Transformation|SetWorldLocation (Variables|Transformation|GetRootComponent) (+ (Transformation|GetWorldLocation (Variables|/Script/Engine.Actor|GetRootComponent (stale _array_element))) "200.000000,200.000000,0.000000") false false)
    (else
      (Development|PrintString "No")
      (CallFunction|TeleportAfterOverlap))))

(event EventBeginPlay
  (bind _outactors (Actor|GetAllActorsOfClass "Lake_C"))
  (bind _output_get (Variables|Default|SetLakesArray _outactors))
  (for (_ _array_index) _output_get
    _)
  (bind _output_get_2 (Variables|Default|SetNumberOfLakes (+ _array_index 1)))
  (Development|PrintString (Utilities|String|ToString(Integer) _output_get_2)))

(event EventTick
  (params (DeltaSeconds :type Float%20%28single-precision%29))
  (bind _npc (Variables|Default|GetNPC))
  (if (Variables|Default|GetLakeTeleporting?)
    (if (Collision|IsOverlappingActor (stale OnComponentBeginOverlap(Box) OverlappedComponent) _npc :!class /Script/Engine.PrimitiveComponent)
      (if (not (> (Math|Vector|VectorLength (Transformation|GetVelocity _npc)) 0.0))
        (if (== (Variables|Default|GetNumberOfLakes) (Variables|Default|GetID))
          _
          (else
            (Transformation|SetWorldLocation (Variables|/Script/Engine.Actor|GetRootComponent _npc) (Variables|Default|GetNextLakeLocation) false false)))
        (Variables|Default|SetLakeTeleporting? false)))))

(fn ConstructionScript)

(fn ChangeTPLocationAfterTeleporting)