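; Boss actor that attacks the player with either a thrown water ball or a wind blow, chosen by whether the player overlaps its floor trigger.
; PawnSensing starts attacks behind busy and cooldown flags, while a looping timer yaws the boss toward the player whenever a tick counter has cleared sight.
; Timelines lerp the ball to the captured position, leaving a puddle, or push the player away when blowing.
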(event OnSeePawn(PawnSensing)
  (params (Pawn :type Pawn%20Object%20Reference))
  (Variables|Default|SetChecking 0)
  (Variables|Default|SetSeesPlayer? true)
  (Development|PrintString "Boss sees player")
  (if (not (Variables|Default|GetIsDoingSomething?))
    (if (Variables|Default|GetisOnFloor)
      (if (Variables|Default|GetCanWater?)
        (Variables|Default|SetIsDoingSomething? true)
        (Variables|Default|SetCanWater? false)
        (CallFunction|ThrowWaterBall))
      (elif (Variables|Default|GetCanBlow?)
        (Variables|Default|SetIsDoingSomething? true)
        (Variables|Default|SetCanBlow? false)
        (CallFunction|Blow)))))

(event OnActorBeginOverlap(floorTriggerBox)
  (params (OverlappedActor :type Actor%20Object%20Reference) (OtherActor :type Actor%20Object%20Reference))
  (Utilities|Casting|CastToBP_ThirdPersonCharacter OtherActor)
  (Variables|Default|SetisOnFloor true))

(event OnActorEndOverlap(floorTriggerBox)
  (params (OverlappedActor :type Actor%20Object%20Reference) (OtherActor :type Actor%20Object%20Reference))
  (Utilities|Casting|CastToBP_ThirdPersonCharacter OtherActor)
  (Variables|Default|SetisOnFloor false))

(event Custom|ThrowWaterBall
  (bind _returnvalue (Transformation|GetActorLocation))
  (Variables|Default|SetIsSwinging? true)
  (Utilities|FlowControl|Delay 1.3)
  ;[1 1 1] Water ball
  (Audio|PlaySoundatLocation "/Game/Sounds/Boss/STOMP_CUE.STOMP_CUE" (Transformation|GetWorldLocation (Variables|Default|Getbroom)) "0, 0, 0" 1.0 1.0 0.0 0 0 0 0)
  (Utilities|FlowControl|Delay 0.7)
  (Variables|Default|SetEndLocation (- (Transformation|GetActorLocation (stale OnSeePawn(PawnSensing) Pawn)) "0,0,90.000000"))
  (bind _returnvalue_2 (Game|SpawnActorfromClass "/Game/Boss/BP_WaterBall.BP_WaterBall_C" (Math|Conversions|ToTransform(Vector) _returnvalue) "Undefined" 0 0))
  (Audio|PlaySoundatLocation "/Game/Sounds/Boss/THROW_CUE.THROW_CUE" (Transformation|GetActorLocation (stale OnSeePawn(PawnSensing) Pawn)) "0, 0, 0" 1.0 1.0 0.0 0 0 0 0)
  (bind _alpha (Timeline|WaterBallMove PlayFromStart)
    (:Update
      (Transformation|SetActorLocation _returnvalue_2 (Math|Vector|Lerp(Vector) _returnvalue (Variables|Default|GetEndLocation) _alpha) false false))
    (:Finished
      (Actor|DestroyActor _returnvalue_2)
      (CallFunction|MakeWaterPuddle)
      (Audio|PlaySoundatLocation "/Game/Sounds/Boss/WATER_SPLASH_CUE.WATER_SPLASH_CUE" (Math|Vector|Lerp(Vector) _returnvalue (Variables|Default|GetEndLocation) _alpha) "0, 0, 0" 1.0 1.0 0.0 0 0 0 0)
      (Variables|Default|SetIsDoingSomething? false)
      (Variables|Default|SetIsSwinging? false)
      (Utilities|FlowControl|Delay 7.0)
      (Variables|Default|SetCanWater? true))))

(event Custom|MakeWaterPuddle
  ;[1 1 1] Water ball
  (Game|SpawnActorfromClass "/Game/Blueprints/BP_Puddle.BP_Puddle_C" (Math|Conversions|ToTransform(Vector) (Variables|Default|GetEndLocation)) "Undefined" 0 0))

(event Custom|Blow
  (bind _returnvalue (Game|GetPlayerCharacter 0))
  (bind _returnvalue_2 (Transformation|GetActorLocation _returnvalue))
  (Utilities|FlowControl|Delay 3.0)
  (Variables|Default|SetIsBlowing? true)
  ;[1 1 1] Blowing
  (Audio|PlaySoundatLocation "/Game/Sounds/Boss/WIND_BLOW_CUE.WIND_BLOW_CUE" (Transformation|GetWorldLocation (Variables|Character|GetMesh)) "0, 0, 0" 1.0 1.0 0.0 0 0 0 0)
  (Timeline|Blowing PlayFromStart
    (:Update
      (Transformation|SetActorLocation _returnvalue (+ _returnvalue_2 (* (* (Math|Vector|Normalize (- _returnvalue_2 (Transformation|GetActorLocation))) (Variables|Default|GetBlowing%20Factor)) (Utilities|Time|GetWorldDeltaSeconds))) true false))
    (:Finished
      (Variables|Default|SetIsDoingSomething? false)
      (Variables|Default|SetIsBlowing? false)
      (Utilities|FlowControl|Delay 7.0)
      (Variables|Default|SetCanBlow? true))))

(event Custom|Rotate
  (bind _returnvalue (Transformation|GetActorRotation))
  (bind (_roll _pitch) (Math|Rotator|BreakRotator _returnvalue))
  (if (not (Variables|Default|GetSeesPlayer?))
    (Development|PrintString "Hello")
    (Transformation|SetActorRotation (Math|Rotator|MakeRotator _roll _pitch (.Yaw (Math|Rotator|BreakRotator (Math|Rotator|FindLookatRotation (Transformation|GetActorLocation) (Transformation|GetActorLocation (Game|GetPlayerCharacter 0)))))))))

(event EventBeginPlay
  (Utilities|Time|SetTimerbyFunctionName 0 "Rotate" 1.0 true))

(event Collision|EventActorBeginOverlap
  (params (OtherActor :type Actor%20Object%20Reference)))

(event EventTick
  (params (DeltaSeconds :type Float%20%28single-precision%29))
  (bind _output_get (Variables|Default|SetChecking (+ (Variables|Default|GetChecking) 1)))
  (if (> _output_get 50)
    (Variables|Default|SetSeesPlayer? false)))

(fn ConstructionScript)